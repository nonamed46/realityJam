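; Teleporter actor that sends the first-person player to a linked Target's TPSpot on overlapping TeleporterArea, preserving speed like a portal.
; It records entry speed, moves the character and sets controller yaw to the spot's facing.
; Velocity is then zeroed and the character launched along the spot's forward vector at that speed.
; The character's CanTeleport flag gates re-entry until its ResetTeleport handles it.
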(event OnComponentBeginOverlap(TeleporterArea)
  (params (OverlappedComponent :type Primitive%20Component%20Object%20Reference) (OtherActor :type Actor%20Object%20Reference) (OtherComp :type Primitive%20Component%20Object%20Reference) (OtherBodyIndex :type Integer) (bFromSweep :type Boolean) (SweepResult :type Hit%20Result%20Structure%20%28by%20ref%29))
  (bind _target (Variables|Default|GetTarget))
  (bind _tp_spot (Variables|/Game/Blueprints/Teleporter1.Teleporter1_C|GetTP_Spot _target))
  (bind _returnvalue (Transformation|GetWorldTransform _tp_spot))
  (Utilities|FlowControl|Sequence
    (:then_0
      (Variables|Default|SetPlayerVelocity (Math|Vector|VectorLength (Transformation|GetVelocity OtherActor))))
    (:then_1
      (bind _astestfirst_person_character (Utilities|Casting|CastToTESTFirstPersonCharacter OtherActor))
      (if (Variables|/Game/FirstPersonBP/Blueprints/TESTFirstPersonCharacter.TESTFirstPersonCharacter_C|GetCanTeleport? _astestfirst_person_character)
        (Variables|/Game/FirstPersonBP/Blueprints/TESTFirstPersonCharacter.TESTFirstPersonCharacter_C|SetCanTeleport? _astestfirst_person_character false)
        (Pawn|SetControlRotation (Game|GetPlayerController 0) (Math|Rotator|MakeRotator (.roll (Transformation|GetActorRotation _astestfirst_person_character)) (.pitch (Transformation|GetActorRotation _astestfirst_person_character)) (.yaw (.rotation _returnvalue))))
        (Transformation|SetActorLocation _astestfirst_person_character (.location _returnvalue) false true)
        (Variables|/Script/Engine.MovementComponent|SetVelocity (Variables|/Script/Engine.Character|GetCharacterMovement _astestfirst_person_character) "0, 0, 0")
        (Character|LaunchCharacter _astestfirst_person_character (* (Math|Vector|Normalize (Math|Vector|GetForwardVector _tp_spot)) (Variables|Default|GetPlayerVelocity)) false false)
        (Default|ResetTeleport _astestfirst_person_character)))))

(fn ConstructionScript)