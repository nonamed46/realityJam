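; Lever actor that the first-person player uses to shift every Cube01, Cube02 and Cube03 actor in the level between two positions.
; A trigger box overlap gates UseLever, and an IsActive flag blocks reuse until the lever's rotation timeline finishes.
; Each use fetches cubes by class, and a FlipFlop per class alternates instantly adding or subtracting the MoveX/Y/Z offsets.
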(event OnComponentBeginOverlap(TriggerBox)
  (params (OverlappedComponent :type Primitive%20Component%20Object%20Reference) (OtherActor :type Actor%20Object%20Reference) (OtherComp :type Primitive%20Component%20Object%20Reference) (OtherBodyIndex :type Integer) (bFromSweep :type Boolean) (SweepResult :type Hit%20Result%20Structure%20%28by%20ref%29))
  ;[1 1 1] Overlap Events check if Player is in Range of Lever or has left activation Range
  (Utilities|Casting|CastToFirstPersonCharacter OtherActor)
  (Variables|Default|SetcanUseLever? true))

(event OnComponentEndOverlap(TriggerBox)
  (params (OverlappedComponent :type Primitive%20Component%20Object%20Reference) (OtherActor :type Actor%20Object%20Reference) (OtherComp :type Primitive%20Component%20Object%20Reference) (OtherBodyIndex :type Integer))
  ;[1 1 1] Overlap Events check if Player is in Range of Lever or has left activation Range
  (Utilities|Casting|CastToFirstPersonCharacter OtherActor)
  (Variables|Default|SetcanUseLever? false))

(event Custom|UseLever
  (bind _lever (Variables|Default|GetLever))
  (bind _returnvalue (Transformation|GetWorldRotation _lever))
  ;[0 1 0.25] Use Lever
  ;;[1 1 1] Checks if Player can use Lever and if Lever is currently in Use
  (if (Variables|Default|GetcanUseLever?)
    (if (not (Variables|Default|GetisActive?))
      (Variables|Default|SetisActive? true)
      (Utilities|FlowControl|Sequence
        (:then_0
          ;;[1 1 1] Gets all Cubes by Class. Switches between 2 Positions by Adding/Subtracting the Move Variables to Positions.
          (bind _outactors (Actor|GetAllActorsOfClass "/Game/Blueprints/Shapes/cube01_BP.cube01_BP_C"))
          (Utilities|FlowControl|FlipFlop
            (:A
              (CallFunction|MoveCubesA _outactors))
            (:B
              (CallFunction|MoveCubesB _outactors))))
        (:then_1
          (bind _outactors_2 (Actor|GetAllActorsOfClass "/Game/Blueprints/Shapes/cube02_BP.cube02_BP_C"))
          (Utilities|FlowControl|FlipFlop
            (:A
              (CallFunction|MoveCubesA _outactors_2))
            (:B
              (CallFunction|MoveCubesB _outactors_2))))
        (:then_2
          (bind _outactors_3 (Actor|GetAllActorsOfClass "/Game/Blueprints/Shapes/cube03_BP.cube03_BP_C"))
          (Utilities|FlowControl|FlipFlop
            (:A
              (CallFunction|MoveCubesA _outactors_3))
            (:B
              (CallFunction|MoveCubesB _outactors_3))))
        (:then_3
          ;;[1 1 1] Starts Lever Animation. Resets IsActive? on Finish.
          (bind _y_rotation (Timeline|Timeline_0 PlayFromStart)
            (:Update
              (Transformation|SetWorldRotation _lever (Math|Rotator|MakeRotator (.roll _returnvalue) _y_rotation (.yaw _returnvalue)) false false))
            (:Finished
              (Variables|Default|SetisActive? false))))))))

(fn ConstructionScript)

(fn MoveCubesA
  (params (CubeArray :type Array%20of%20Actor%20Object%20References))
  (for _array_element CubeArray
    (Transformation|SetActorLocation _array_element (Math|Vector|MakeVector (+ (.x (Transformation|GetActorLocation _array_element)) (Variables|Default|GetMoveX)) (+ (.y (Transformation|GetActorLocation _array_element)) (Variables|Default|GetMoveY)) (+ (.z (Transformation|GetActorLocation _array_element)) (Variables|Default|GetMoveZ))) false false)))

(fn MoveCubesB
  (params (CubeArray :type Array%20of%20Actor%20Object%20References))
  (for _array_element CubeArray
    (Transformation|SetActorLocation _array_element (Math|Vector|MakeVector (- (.x (Transformation|GetActorLocation _array_element)) (Variables|Default|GetMoveX)) (- (.y (Transformation|GetActorLocation _array_element)) (Variables|Default|GetMoveY)) (- (.z (Transformation|GetActorLocation _array_element)) (Variables|Default|GetMoveZ))) false false)))