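; Lever actor that mirrors all puzzle pyramids when the first-person player uses it from inside its trigger box.
; UseLever, gated by range and an IsActive lock, negates the scale of every actor of five Pyramid classes via MirrorPyramids.
; A timeline then animates the lever's pitch and clears the lock when finished.
; Entering the trigger shows the pyramid streaming level and hides cube and plank levels; leaving hides all three.
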(event OnComponentBeginOverlap(TriggerBox)
  (params (OverlappedComponent :type Primitive%20Component%20Object%20Reference) (OtherActor :type Actor%20Object%20Reference) (OtherComp :type Primitive%20Component%20Object%20Reference) (OtherBodyIndex :type Integer) (bFromSweep :type Boolean) (SweepResult :type Hit%20Result%20Structure%20%28by%20ref%29))
  ;[1 1 1] Overlap Events check if Player is in Range of Lever or has left activation Range
  (Utilities|Casting|CastToFirstPersonCharacter OtherActor)
  (Variables|Default|SetcanUseLever? true)
  (CallFunction|ShowPyrmids))

(event OnComponentEndOverlap(TriggerBox)
  (params (OverlappedComponent :type Primitive%20Component%20Object%20Reference) (OtherActor :type Actor%20Object%20Reference) (OtherComp :type Primitive%20Component%20Object%20Reference) (OtherBodyIndex :type Integer))
  ;[1 1 1] Overlap Events check if Player is in Range of Lever or has left activation Range
  (Utilities|Casting|CastToFirstPersonCharacter OtherActor)
  (Variables|Default|SetcanUseLever? false)
  (CallFunction|HidePyramids))

(event Custom|UseLever
  (bind _lever (Variables|Default|GetLever))
  (bind _returnvalue (Transformation|GetWorldRotation _lever))
  ;[1 0.5773 0.4262] Use Lever
  ;;[1 1 1] Checks if Player can use Lever and Starts Sequence if Lever is not active
  (if (Variables|Default|GetcanUseLever?)
    (if (not (Variables|Default|GetisActive?))
      (Variables|Default|SetisActive? true)
      (Utilities|FlowControl|Sequence
        (:then_0
          ;;[1 1 1] Gets all Pyramids by class and mirrors them
          (bind _outactors (Actor|GetAllActorsOfClass "/Game/Blueprints/Shapes/pyramid01_BP.pyramid01_BP_C"))
          (CallFunction|MirrorPyramids _outactors))
        (:then_1
          (bind _outactors_2 (Actor|GetAllActorsOfClass "/Game/Blueprints/Shapes/pyramid02_BP.pyramid02_BP_C"))
          (CallFunction|MirrorPyramids _outactors_2))
        (:then_2
          (bind _outactors_3 (Actor|GetAllActorsOfClass "/Game/Blueprints/Shapes/pyramid03_BP.pyramid03_BP_C"))
          (CallFunction|MirrorPyramids _outactors_3))
        (:then_3
          (bind _outactors_4 (Actor|GetAllActorsOfClass "/Game/Blueprints/Shapes/pyramid04_BP.pyramid04_BP_C"))
          (CallFunction|MirrorPyramids _outactors_4))
        (:then_4
          (bind _outactors_5 (Actor|GetAllActorsOfClass "/Game/Blueprints/Shapes/pyramid05_BP.pyramid05_BP_C"))
          (CallFunction|MirrorPyramids _outactors_5))
        (:then_5
          ;;[1 1 1] Plays Lever Animation. On Finished resets IsActive?
          (bind _y_rotation (Timeline|LeverAnim01 PlayFromStart)
            (:Update
              (Transformation|SetWorldRotation _lever (Math|Rotator|MakeRotator (.roll _returnvalue) _y_rotation (.yaw _returnvalue)) false false))
            (:Finished
              (Variables|Default|SetisActive? false))))))))

(event Custom|ShowPyrmids
  (Variables|/Script/Engine.LevelStreaming|SetbShouldBeVisible (Class|GameplayStatics|GetStreamingLevel "Josef_CubeStreaming") false)
  (Variables|/Script/Engine.LevelStreaming|SetbShouldBeVisible (Class|GameplayStatics|GetStreamingLevel "Josef_PlankStreaming") false)
  (Variables|/Script/Engine.LevelStreaming|SetbShouldBeVisible (Class|GameplayStatics|GetStreamingLevel "Josef_PyramidStreaming") true))

(event Custom|HidePyramids
  (Variables|/Script/Engine.LevelStreaming|SetbShouldBeVisible (Class|GameplayStatics|GetStreamingLevel "Josef_CubeStreaming") false)
  (Variables|/Script/Engine.LevelStreaming|SetbShouldBeVisible (Class|GameplayStatics|GetStreamingLevel "Josef_PlankStreaming") false)
  (Variables|/Script/Engine.LevelStreaming|SetbShouldBeVisible (Class|GameplayStatics|GetStreamingLevel "Josef_PyramidStreaming") false))

(fn ConstructionScript)

(fn MirrorPyramids
  (params (PyramidArray :type Array%20of%20Actor%20Object%20References))
  (for _array_element PyramidArray
    (Transformation|SetActorTransform _array_element (Math|Transform|MakeTransform (.location (Transformation|GetActorTransform _array_element)) (.rotation (Transformation|GetActorTransform _array_element)) (* (.scale (Transformation|GetActorTransform _array_element)) -1.0)))))