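; Wheel actor that spins, and rotates the level's plank actors with it, while the first-person character stands in its trigger box.
; On BeginPlay it gathers all Plank01 to Plank04 Blueprint actors into four arrays.
; Trigger overlaps toggle the turning flag, which Tick checks to yaw every plank through RotatePlank and pitch the Rad mesh, both at TurnRate scaled by delta time.
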(event OnComponentBeginOverlap(TriggerBox)
  (params (OverlappedComponent :type Primitive%20Component%20Object%20Reference) (OtherActor :type Actor%20Object%20Reference) (OtherComp :type Primitive%20Component%20Object%20Reference) (OtherBodyIndex :type Integer) (bFromSweep :type Boolean) (SweepResult :type Hit%20Result%20Structure%20%28by%20ref%29))
  (Utilities|Casting|CastToFirstPersonCharacter OtherActor)
  (Variables|Default|SetcanTurnWheel? true)
  (Variables|Default|SetisTurningWheel? true))

(event OnComponentEndOverlap(TriggerBox)
  (params (OverlappedComponent :type Primitive%20Component%20Object%20Reference) (OtherActor :type Actor%20Object%20Reference) (OtherComp :type Primitive%20Component%20Object%20Reference) (OtherBodyIndex :type Integer))
  (Utilities|Casting|CastToFirstPersonCharacter OtherActor)
  (Variables|Default|SetcanTurnWheel? false)
  (Variables|Default|SetisTurningWheel? false))

(event EventBeginPlay
  (Utilities|FlowControl|Sequence
    (:then_0
      (bind _outactors (Actor|GetAllActorsOfClass "/Game/Blueprints/Shapes/plank04_BP.plank04_BP_C"))
      (Utilities|Array|AppendArray (Variables|Default|GetPlank04Array) _outactors))
    (:then_1
      (bind _outactors_2 (Actor|GetAllActorsOfClass "/Game/Blueprints/Shapes/plank03_BP.plank03_BP_C"))
      (Utilities|Array|AppendArray (Variables|Default|GetPlank03Array) _outactors_2))
    (:then_2
      (bind _outactors_3 (Actor|GetAllActorsOfClass "/Game/Blueprints/Shapes/plank02_BP.plank02_BP_C"))
      (Utilities|Array|AppendArray (Variables|Default|GetPlank02Array) _outactors_3))
    (:then_3
      (bind _outactors_4 (Actor|GetAllActorsOfClass "/Game/Blueprints/Shapes/plank01_BP.plank01_BP_C"))
      (Utilities|Array|AppendArray (Variables|Default|GetPlank01Array) _outactors_4))))

(event EventTick
  (params (DeltaSeconds :type Float%20%28single-precision%29))
  (bind _rad (Variables|Default|GetRad))
  (bind _returnvalue (Transformation|GetWorldRotation _rad))
  (if (Variables|Default|GetisTurningWheel?)
    (Utilities|FlowControl|Sequence
      (:then_0
        (CallFunction|RotatePlank (Variables|Default|GetPlank04Array)))
      (:then_1
        (CallFunction|RotatePlank (Variables|Default|GetPlank03Array)))
      (:then_2
        (CallFunction|RotatePlank (Variables|Default|GetPlank02Array)))
      (:then_3
        (CallFunction|RotatePlank (Variables|Default|GetPlank01Array))
        (Transformation|SetWorldRotation _rad (Math|Rotator|MakeRotator (.roll _returnvalue) (+ (.pitch _returnvalue) (* (Utilities|Time|GetWorldDeltaSeconds) (Variables|Default|GetTurnRate))) (.yaw _returnvalue)) false false)))))

(fn ConstructionScript)

(fn RotatePlank
  (params (Array :type Array%20of%20Actor%20Object%20References))
  (for _array_element Array
    (Transformation|SetActorRotation _array_element (Math|Rotator|MakeRotator (.roll (Transformation|GetActorRotation _array_element)) (.pitch (Transformation|GetActorRotation _array_element)) (+ (.yaw (Transformation|GetActorRotation _array_element)) (* (Utilities|Time|GetWorldDeltaSeconds) (Variables|Default|GetTurnRate)))))))