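; Test lever actor that moves every Cube01, Cube02 and Cube03 actor in the level when used.
; Its trigger box enables use while the first-person character overlaps, and entering also makes all cubes visible and collidable.
; UseLever calls MoveCube on each cube, plays a sound and pitches the lever via a timeline, blocking reuse until it finishes.
; HideCubes, the FlipFlop move alternative and level-streaming visibility logic are unwired.
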(event OnComponentBeginOverlap(TriggerBox)
  (params (OverlappedComponent :type Primitive%20Component%20Object%20Reference) (OtherActor :type Actor%20Object%20Reference) (OtherComp :type Primitive%20Component%20Object%20Reference) (OtherBodyIndex :type Integer) (bFromSweep :type Boolean) (SweepResult :type Hit%20Result%20Structure%20%28by%20ref%29))
  ;[1 1 1] Overlap Events check if Player is in Range of Lever or has left activation Range
  (Utilities|Casting|CastToTESTFirstPersonCharacter OtherActor)
  (Variables|Default|SetcanUseLever? true)
  (CallFunction|ShowCubes))

(event OnComponentEndOverlap(TriggerBox)
  (params (OverlappedComponent :type Primitive%20Component%20Object%20Reference) (OtherActor :type Actor%20Object%20Reference) (OtherComp :type Primitive%20Component%20Object%20Reference) (OtherBodyIndex :type Integer))
  ;[1 1 1] Overlap Events check if Player is in Range of Lever or has left activation Range
  (Utilities|Casting|CastToTESTFirstPersonCharacter OtherActor)
  (Variables|Default|SetcanUseLever? false))

(event Custom|UseLever
  (bind _lever (Variables|Default|GetLever))
  (bind _returnvalue (Transformation|GetWorldRotation _lever))
  ;[0 1 0.25] Use Lever
  ;;[1 1 1] Checks if Player can use Lever and if Lever is currently in Use
  (if (Variables|Default|GetcanUseLever?)
    (if (not (Variables|Default|GetisActive?))
      (Variables|Default|SetisActive? true)
      (Utilities|FlowControl|Sequence
        (:then_0
          ;;[1 1 1] Gets all Cubes by Class. Switches between 2 Positions by Adding/Subtracting the Move Variables to Positions.
          (bind _outactors (Actor|GetAllActorsOfClass "/Game/Blueprints/Shapes/cube01_BP.cube01_BP_C"))
          (for _array_element _outactors
            (Default|MoveCube _array_element)))
        (:then_1
          (bind _outactors_2 (Actor|GetAllActorsOfClass "/Game/Blueprints/Shapes/cube02_BP.cube02_BP_C"))
          (for _array_element_2 _outactors_2
            (Default|MoveCube _array_element_2)))
        (:then_2
          (bind _outactors_3 (Actor|GetAllActorsOfClass "/Game/Blueprints/Shapes/cube03_BP.cube03_BP_C"))
          (for _array_element_3 _outactors_3
            (Default|MoveCube _array_element_3)))
        (:then_3
          ;;[1 1 1] Starts Lever Animation. Resets IsActive? on Finish.
          (Audio|PlaySoundatLocation "/Game/Audio/Lever01.Lever01" (Transformation|GetWorldLocation _lever) "0, 0, 0" 1.0 1.0 0.0 0 0 0)
          (bind _y_rotation (Timeline|Timeline_0 PlayFromStart)
            (:Update
              (Transformation|SetWorldRotation _lever (Math|Rotator|MakeRotator (.roll _returnvalue) _y_rotation (.yaw _returnvalue)) false false))
            (:Finished
              (Variables|Default|SetisActive? false))))))))

(event Custom|ShowCubes
  (Utilities|FlowControl|Sequence
    (:then_0
      (bind _outactors (Actor|GetAllActorsOfClass "/Game/Blueprints/Shapes/cube01_BP.cube01_BP_C"))
      (for _array_element _outactors
        (Rendering|SetVisibility (Variables|/Game/Blueprints/Shapes/cube01_BP.cube01_BP_C|GetStaticMesh _array_element) true false)
        (Collision|SetActorEnableCollision _array_element true)))
    (:then_1
      (bind _outactors_2 (Actor|GetAllActorsOfClass "/Game/Blueprints/Shapes/cube02_BP.cube02_BP_C"))
      (for _array_element_2 _outactors_2
        (Rendering|SetVisibility (Variables|/Script/Engine.Actor|GetRootComponent _array_element_2) true false)
        (Collision|SetActorEnableCollision _array_element_2 true)))
    (:then_2
      (bind _outactors_3 (Actor|GetAllActorsOfClass "/Game/Blueprints/Shapes/cube03_BP.cube03_BP_C"))
      (for _array_element_3 _outactors_3
        (Rendering|SetVisibility (Variables|/Script/Engine.Actor|GetRootComponent _array_element_3) true false)
        (Collision|SetActorEnableCollision _array_element_3 true)))))

(event Custom|HideCubes
  (Utilities|FlowControl|Sequence
    (:then_0
      (bind _outactors (Actor|GetAllActorsOfClass "/Game/Blueprints/Shapes/cube01_BP.cube01_BP_C"))
      (for _array_element _outactors
        (Rendering|SetVisibility (Variables|/Game/Blueprints/Shapes/cube01_BP.cube01_BP_C|GetStaticMesh _array_element) false false)
        (Collision|SetActorEnableCollision _array_element false)))
    (:then_1
      (bind _outactors_2 (Actor|GetAllActorsOfClass "/Game/Blueprints/Shapes/cube02_BP.cube02_BP_C"))
      (for _array_element_2 _outactors_2
        (Rendering|SetVisibility (Variables|/Script/Engine.Actor|GetRootComponent _array_element_2) false false)
        (Collision|SetActorEnableCollision _array_element_2 false)))
    (:then_2
      (bind _outactors_3 (Actor|GetAllActorsOfClass "/Game/Blueprints/Shapes/cube03_BP.cube03_BP_C"))
      (for _array_element_3 _outactors_3
        (Rendering|SetVisibility (Variables|/Script/Engine.Actor|GetRootComponent _array_element_3) false false)
        (Collision|SetActorEnableCollision _array_element_3 false)))))

(fn ConstructionScript)

(fn MoveCubesA
  (params (CubeArray :type Array%20of%20Actor%20Object%20References))
  (for _array_element CubeArray
    (Transformation|SetActorLocation _array_element (Math|Vector|MakeVector (+ (.x (Transformation|GetActorLocation _array_element)) (Variables|Default|GetMoveX)) (+ (.y (Transformation|GetActorLocation _array_element)) (Variables|Default|GetMoveY)) (+ (.z (Transformation|GetActorLocation _array_element)) (Variables|Default|GetMoveZ))) false false)))

(fn MoveCubesB
  (params (CubeArray :type Array%20of%20Actor%20Object%20References))
  (for _array_element CubeArray
    (Transformation|SetActorLocation _array_element (Math|Vector|MakeVector (- (.x (Transformation|GetActorLocation _array_element)) (Variables|Default|GetMoveX)) (- (.y (Transformation|GetActorLocation _array_element)) (Variables|Default|GetMoveY)) (- (.z (Transformation|GetActorLocation _array_element)) (Variables|Default|GetMoveZ))) false false)))