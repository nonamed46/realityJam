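; Gem socket actor that controls a gate, which returns to its starting position once three gems are placed.
; Four seconds after BeginPlay, a timeline moves the gate along Z with a wheel sound.
; CheckForGems takes one held gem from the first-person character per call and reveals its mesh in the socket.
; When all three show, a portal sound plays and the timeline reverses with the wheel sound, cut after a fixed delay.
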(event Custom|CheckForGems
  (bind _gem1 (Variables|Default|GetGem1))
  (bind _gate (Variables|Default|GetGate))
  (bind _gem3 (Variables|Default|GetGem3))
  (bind _gem2 (Variables|Default|GetGem2))
  (bind _relativelocation (Variables|/Script/Engine.SceneComponent|GetRelativeLocation _gate))
  (bind _astestfirst_person_character (Utilities|Casting|CastToTESTFirstPersonCharacter (Game|GetPlayerCharacter 0)))
  (if (Variables|/Game/FirstPersonBP/Blueprints/TESTFirstPersonCharacter.TESTFirstPersonCharacter_C|GetHasGem1? _astestfirst_person_character)
    (Variables|/Game/FirstPersonBP/Blueprints/TESTFirstPersonCharacter.TESTFirstPersonCharacter_C|SetHasGem1? _astestfirst_person_character false)
    (Rendering|SetVisibility _gem1 true false)
    (Audio|PlaySoundatLocation "/Game/Audio/Collected01.Collected01" (Transformation|GetWorldLocation _gem1) "0, 0, 0" 1.0 1.0 0.0 0 0 0)
    (if (Math|Boolean|ANDBoolean (Variables|/Script/Engine.SceneComponent|GetbVisible _gem1) (Variables|/Script/Engine.SceneComponent|GetbVisible _gem2) (Variables|/Script/Engine.SceneComponent|GetbVisible _gem3)) :!label _label
      (Audio|PlaySoundatLocation "/Game/Audio/Portal02.Portal02" (Transformation|GetWorldLocation (Variables|Debug|GetStaticMeshComponent)) "0, 0, 0" 1.0 1.0 0.0 0 0 0)
      (bind _returnvalue (Audio|SpawnSoundatLocation "/Game/Audio/Wheel02_Cue.Wheel02_Cue" (Transformation|GetActorLocation) "0, 0, 0" 1.0 1.0 0.0 0 0))
      (Utilities|FlowControl|Sequence
        (:then_0
          (bind _z_pos (Timeline|Timeline_0 ReverseFromEnd)
            (:Update
              (Transformation|SetRelativeLocation _gate (Math|Vector|MakeVector (.x _relativelocation) (.y _relativelocation) _z_pos) false false))
            (:Finished
              (Utilities|IsValid (stale EventBeginPlay _returnvalue)
                (:Is%20Valid
                  (Audio|Components|Audio|FadeOut (stale EventBeginPlay _returnvalue) 0.0 0.0 :!class /Script/Engine.AudioComponent))))))
        (:then_1
          (Utilities|FlowControl|Delay 1e+01)
          (Utilities|IsValid _returnvalue
            (:Is%20Valid
              (Audio|Components|Audio|FadeOut _returnvalue 0.0 0.0 :!class /Script/Engine.AudioComponent))))))
    (elif (Variables|/Game/FirstPersonBP/Blueprints/TESTFirstPersonCharacter.TESTFirstPersonCharacter_C|GetHasGem2? _astestfirst_person_character)
      (Variables|/Game/FirstPersonBP/Blueprints/TESTFirstPersonCharacter.TESTFirstPersonCharacter_C|SetHasGem2? _astestfirst_person_character false)
      (Rendering|SetVisibility _gem2 true false)
      (Audio|PlaySoundatLocation "/Game/Audio/Collected01.Collected01" (Transformation|GetWorldLocation _gem2) "0, 0, 0" 1.0 1.0 0.0 0 0 0)
      (goto _label)
      (elif (Variables|/Game/FirstPersonBP/Blueprints/TESTFirstPersonCharacter.TESTFirstPersonCharacter_C|GetHasGem3? _astestfirst_person_character)
        (Variables|/Game/FirstPersonBP/Blueprints/TESTFirstPersonCharacter.TESTFirstPersonCharacter_C|SetHasGem3? _astestfirst_person_character false)
        (Rendering|SetVisibility _gem3 true false)
        (Audio|PlaySoundatLocation "/Game/Audio/Collected01.Collected01" (Transformation|GetWorldLocation _gem3) "0, 0, 0" 1.0 1.0 0.0 0 0 0)
        (goto _label)))))

(event EventBeginPlay
  (bind _gate (Variables|Default|GetGate))
  (bind _relativelocation (Variables|/Script/Engine.SceneComponent|GetRelativeLocation _gate))
  (Utilities|FlowControl|Delay 4.0)
  (bind _returnvalue (Audio|SpawnSoundatLocation "/Game/Audio/Wheel02_Cue.Wheel02_Cue" (Transformation|GetActorLocation) "0, 0, 0" 1.0 1.0 0.0 0 0))
  (bind _z_pos (Timeline|Timeline_0 Play)
    (:Update
      (Transformation|SetRelativeLocation _gate (Math|Vector|MakeVector (.x _relativelocation) (.y _relativelocation) _z_pos) false false))
    (:Finished
      (Utilities|IsValid _returnvalue
        (:Is%20Valid
          (Audio|Components|Audio|FadeOut _returnvalue 0.0 0.0 :!class /Script/Engine.AudioComponent))))))

(fn ConstructionScript)