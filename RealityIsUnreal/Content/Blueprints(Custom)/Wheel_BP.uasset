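; Wheel_BP is a wheel actor that slowly turns while the first-person character stands inside its box trigger.
; Box overlap events toggle IsTurningWheel and CanTurnWheel; Tick checks only the former and advances the mesh's world yaw at a constant, delta-time-scaled rate.
; On BeginPlay, each wheel gathers all Wheel_BP actors into AshlarArray and prints their names and indices as debug output.
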(event OnComponentBeginOverlap(Box)
  (params (OverlappedComponent :type Primitive%20Component%20Object%20Reference) (OtherActor :type Actor%20Object%20Reference) (OtherComp :type Primitive%20Component%20Object%20Reference) (OtherBodyIndex :type Integer) (bFromSweep :type Boolean) (SweepResult :type Hit%20Result%20Structure%20%28by%20ref%29))
  (Utilities|Casting|CastToFirstPersonCharacter OtherActor)
  (Variables|Default|SetcanTurnWheel? true)
  (Variables|Default|SetisTurningWheel? true))

(event OnComponentEndOverlap(Box)
  (params (OverlappedComponent :type Primitive%20Component%20Object%20Reference) (OtherActor :type Actor%20Object%20Reference) (OtherComp :type Primitive%20Component%20Object%20Reference) (OtherBodyIndex :type Integer))
  (Utilities|Casting|CastToFirstPersonCharacter OtherActor)
  (Variables|Default|SetcanTurnWheel? false)
  (Variables|Default|SetisTurningWheel? false))

(event EventBeginPlay
  (bind _ashlararray (Variables|Default|GetAshlarArray))
  (bind _outactors (Actor|GetAllActorsOfClass "Wheel_BP_C"))
  (Utilities|Array|AppendArray _ashlararray _outactors)
  (for (_array_element _array_index) _ashlararray
    (Development|PrintString (Utilities|String|Append (Utilities|GetObjectName _array_element) (Utilities|String|ToString(Integer) _array_index))))
  (Development|PrintString "done"))

(event EventTick
  (params (DeltaSeconds :type Float%20%28single-precision%29))
  (bind _staticmesh (Variables|Default|GetStaticMesh))
  (bind _returnvalue (Transformation|GetWorldRotation _staticmesh))
  (if (Variables|Default|GetisTurningWheel?)
    (Transformation|SetWorldRotation _staticmesh (Math|Rotator|MakeRotator (.roll _returnvalue) (.pitch _returnvalue) (+ (.yaw _returnvalue) (* (Utilities|Time|GetWorldDeltaSeconds) 5.0))) false false)))

(fn ConstructionScript)